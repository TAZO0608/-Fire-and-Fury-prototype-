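; Enemy tank Blueprint that wires its barrel, turret, tracks, movement and smoke components into inherited or component functions.
; BeginPlay hands over those references and passes itself to the widget component's HealthBar.
; Input events rotate the root and spring arm for the camera, drive tracks directly or through the movement component, and trigger firing, despite the enemy name.
; Activating the Smoke component plays a fire loop sound at the tank's location.
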(event OnComponentActivated(smoke)
  (params (Component :type Actor%20Component%20Object%20Reference) (bReset :type Boolean))
  (Audio|PlaySoundatLocation "/Game/tank/SFX/Loop__fire.Loop__fire" (Transformation|GetActorLocation)))

(event EventBeginPlay
  (Class|Tank|SettoBarrel (Variables|Default|GetMyBarrel))
  (Class|Tank|SettoTurret (Variables|Default|GetMyTurret))
  (Class|MyMovement|SetTrack (Variables|Default|GetmyMovement) (Variables|Default|GetMyTrack_L) (Variables|Default|GetMyTrack_R))
  (Class|Tank|GetSmoke (Variables|Default|Getsmoke))
  (bind _ashealth_bar (Utilities|Casting|CastToHealthBar (UserInterface|GetUserWidgetObject (Variables|Default|GetWidget))))
  (Variables|/Game/UI/HealthBar.HealthBar_C|Setpercentage _ashealth_bar self))

(event Input|ActionEvents|InputActionFIRE
  (params (Key :type Key%20Structure))
  ;[1 1 1] camara_input
  (:Pressed
    (Class|Tank|FIRE)))

(event Input|AxisEvents|InputAxisAzrimuth
  (params (AxisValue :type Float%20%28single-precision%29))
  ;[1 1 1] camara_input
  (Transformation|AddLocalRotation (Variables|Default|Getroot) (Math|Rotator|MakeRotator 0.0 0.0 AxisValue) false false))

(event Input|AxisEvents|InputAxiselevation
  (params (AxisValue :type Float%20%28single-precision%29))
  ;[1 1 1] camara_input
  (Transformation|AddLocalRotation (Variables|Default|GetSpringArm) (Math|Rotator|MakeRotator 0.0 AxisValue 0.0) false false))

(event Input|AxisEvents|InputAxisleft
  (params (AxisValue :type Float%20%28single-precision%29))
  ;[1 1 1] MOVE_INPUT
  (Class|MyTrack|SetThrottle (Variables|Default|GetMyTrack_L) AxisValue))

(event Input|AxisEvents|InputAxisright
  (params (AxisValue :type Float%20%28single-precision%29))
  ;[1 1 1] MOVE_INPUT
  (Class|MyTrack|SetThrottle (Variables|Default|GetMyTrack_R) AxisValue))

(event Input|AxisEvents|InputAxisForward_Back
  (params (AxisValue :type Float%20%28single-precision%29))
  ;[1 1 1] MOVE_INPUT
  (Class|MyMovement|Moveforward (Variables|Default|GetmyMovement) AxisValue))

(event Input|AxisEvents|InputAxisTurn
  (params (AxisValue :type Float%20%28single-precision%29))
  ;[1 1 1] MOVE_INPUT
  (Class|MyMovement|TurnRight (Variables|Default|GetmyMovement) AxisValue))

(fn ConstructionScript)